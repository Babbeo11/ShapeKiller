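; AI controller for enemies that detects and chases the player, including across possession and unpossession of objects.
; Sight perception fills a detection meter, or resumes a chase directly if already chasing, while hearing triggers investigation.
; Gameplay tags track sight and chase status, and events drive a StateTree between chase, seeking, investigation and routine.
; Looping timers detect forgotten targets and player zone changes; last seen location is extrapolated from target velocity.
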(event OnPerceptionUpdated(AIPerception)
  (params (UpdatedActors :type Array%20of%20Actor%20Object%20References))
  ;[1 0.6771 0.6771] Handle AI Perception
  (for _array_element UpdatedActors
    (if (== _array_element (Game|Player|GetPlayerPawn 0))
      (HandleTarget|SetLastSeenLocation)
      (Utilities|FlowControl|Sequence
        (:then_0
          (bind (_sensed _stimulus) (HandleSenses|CanSenseActor _array_element "NewEnumerator0"))
          (if _sensed
            (HandleSenses|HandleSensedSight _array_element _stimulus)
            (else
              (HandleSenses|HandleLostSight _array_element))))
        (:then_1
          (bind (_sensed_2 _stimulus_2) (HandleSenses|CanSenseActor _array_element "NewEnumerator1"))
          (if _sensed_2
            (HandleSenses|HandleSensedHearing _array_element _stimulus_2))))
      (else
        (Class|KismetSystemLibrary|IsObjectOfSoftClass _array_element "/Game/Blueprints/Pawns/BP_PossessableObject.BP_PossessableObject_C"
          (:True
            (Utilities|Array|AddUnique (Variables|Actors|GetKnownSeenActors) _array_element)))))))

(event Custom|CheckIfForgottenSeenActor
  ;[0.1719 1 0] Check When Actor is Forgotten
  (|SetFilteredActors)
  (if (!= (Utilities|Array|Length (Variables|Actors|GetKnownSeenActors)) (Utilities|Array|Length (Variables|Actors|GetKnownSeenActorsFiltered)))
    (for _array_element (Variables|Actors|GetKnownSeenActors)
      (if (== (Utilities|Array|FindItem (Variables|Actors|GetKnownSeenActorsFiltered) _array_element) -1)
        (if (== _array_element (Variables|Actors|GetTargetActor))
          (HandleSenses|HandleForgotActor _array_element))))))

(event Custom|UpdatePerception
  ;[1 0.6771 0.6771] Handle AI Perception
  (for _array_element (stale OnPerceptionUpdated(AIPerception) UpdatedActors)
    (if (== _array_element (Game|Player|GetPlayerPawn 0))
      (HandleTarget|SetLastSeenLocation)
      (Utilities|FlowControl|Sequence
        (:then_0
          (bind (_sensed _stimulus) (HandleSenses|CanSenseActor _array_element "NewEnumerator0"))
          (if _sensed
            (HandleSenses|HandleSensedSight _array_element _stimulus)
            (else
              (HandleSenses|HandleLostSight _array_element))))
        (:then_1
          (bind (_sensed_2 _stimulus_2) (HandleSenses|CanSenseActor _array_element "NewEnumerator1"))
          (if _sensed_2
            (HandleSenses|HandleSensedHearing _array_element _stimulus_2))))
      (else
        (Class|KismetSystemLibrary|IsObjectOfSoftClass _array_element "/Game/Blueprints/Pawns/BP_PossessableObject.BP_PossessableObject_C"
          (:True
            (Utilities|Array|AddUnique (Variables|Actors|GetKnownSeenActors) _array_element)))))))

(event Custom|CheckZoneChange
  ;[0.1484 0 1] Check When Target Zone Change
  (bind _zonetype (Class|BPIPlayerInfo|GetCurrentZone(Message) (Game|Player|GetPlayerPawn 0)))
  (if (Utilities|Enum|NotEqual(Enum) _zonetype (Variables|TargetInfo|GetZoneType))
    (Variables|TargetInfo|SetZoneType _zonetype)
    (CallFunction|UpdatePerception)))

(event Custom|OnPossesObject
  ;[0 1 0.8594] Handle on posses/unposses enemy behavior, based on if chasing or not, and if can see target
  (Default|SetCurrentZone (Variables|Actors|GetRefCoreCharacter) (Variables|TargetInfo|GetZoneType))
  (if (not (Pure|IsEnemyChasing))
    (Variables|Actors|GetTargetActor
      (:then
        (if (Pure|CanSeeTarget)
          (HandleSenses|RefreshTarget)
          (bind _output_get (Variables|/Game/Blueprints/AI/BP_Enemy.BP_Enemy_C|SetDetectionMeter (Variables|Actors|GetRefEnemy) 1e+02))
          (Class|BPIDetectionWidget|OnDetection(Message) (Variables|Actors|GetRefEnemy) _output_get)
          (else
            (Class|BPIDetectionSystem|ActivateDetection(Message) (Variables|Actors|GetRefEnemy) (Variables|Actors|GetTargetActor)))))
      (:else
        (CallFunction|UpdatePerception)))
    (else
      (HandleSenses|RefreshTarget)
      (if (Pure|CanSeeTarget)
        (Gameplay|StateTree|SendStateTreeEvent (Variables|Default|GetStateTreeAI) (Utilities|Struct|MakeStateTreeEvent "(TagName=\"StateTree.Chase\")" "None" "None") :!class /Script/GameplayStateTreeModule.StateTreeComponent)
        (else
          (Class|BPIDetectionSystem|DisableDetection(Message) (Variables|Actors|GetRefEnemy)))))))

(event Custom|OnUnpossesObject
  ;[0 1 0.8594] Handle on posses/unposses enemy behavior, based on if chasing or not, and if can see target
  (Default|SetCurrentZone (Variables|Actors|GetRefCoreCharacter) (Variables|TargetInfo|GetZoneType))
  (if (not (Pure|IsEnemyChasing))
    (Variables|Actors|GetTargetActor
      (:then
        (if (Pure|CanSeeTarget)
          (HandleSenses|RefreshTarget)
          (bind _output_get (Variables|/Game/Blueprints/AI/BP_Enemy.BP_Enemy_C|SetDetectionMeter (Variables|Actors|GetRefEnemy) 1e+02))
          (Class|BPIDetectionWidget|OnDetection(Message) (Variables|Actors|GetRefEnemy) _output_get)
          (else
            (Class|BPIDetectionSystem|ActivateDetection(Message) (Variables|Actors|GetRefEnemy) (Variables|Actors|GetTargetActor)))))
      (:else
        (CallFunction|UpdatePerception)))
    (else
      (HandleSenses|RefreshTarget)
      (if (Pure|CanSeeTarget)
        (Gameplay|StateTree|SendStateTreeEvent (Variables|Default|GetStateTreeAI) (Utilities|Struct|MakeStateTreeEvent "(TagName=\"StateTree.Chase\")" "None" "None") :!class /Script/GameplayStateTreeModule.StateTreeComponent)
        (else
          (Class|BPIDetectionSystem|DisableDetection(Message) (Variables|Actors|GetRefEnemy)))))))

(event EventUnPossess
  (params (UnpossessedPawn :type Pawn%20Object%20Reference))
  ;[1 0 0.4922] Clear Timers
  (Utilities|Time|ClearandInvalidateTimerbyHandle (Variables|Timers|GetCheckForgottenActorsTimer))
  (Utilities|Time|ClearandInvalidateTimerbyHandle (Variables|Timers|GetCheckZoneChangeTimer)))

(event EventChaseonDetection
  ;[0 1 0.2266] Chase On Detection
  (Gameplay|StateTree|SendStateTreeEvent (Variables|Default|GetStateTreeAI) (Utilities|Struct|MakeStateTreeEvent "(TagName=\"StateTree.Chase\")" "None" "None") :!class /Script/GameplayStateTreeModule.StateTreeComponent)
  (GameplayTags|AddGameplayTag (Variables|/Game/Blueprints/AI/BP_Enemy.BP_Enemy_C|GetTagContainer (Variables|Actors|GetRefEnemy)) "(TagName=\"Enemy.Status.Chasing\")" :!class /Script/GameplayTags.BlueprintGameplayTagLibrary))

(event EventPossess
  (params (PossessedPawn :type Pawn%20Object%20Reference))
  (Utilities|FlowControl|DelayUntilNextTick)
  (Class|BrainComponent|RestartLogic (Variables|Default|GetStateTreeAI))
  (Base|GetRef PossessedPawn)
  (Base|SetTimers)
  (EventDispatchers|BindEventtoOnPossess (Variables|Actors|GetRefCoreCharacter) (EventDispatchers|CreateEvent :!event Custom|OnPossesObject))
  (EventDispatchers|BindEventtoOnUnpossess (Variables|Actors|GetRefCoreCharacter) (EventDispatchers|CreateEvent :!event Custom|OnUnpossesObject)))

(fn ConstructionScript)

(fn CanSenseActor
  (params (Actor :type Actor%20Object%20Reference) (Sense :type E_AISense%20Enum :default "NewEnumerator0"))
  ;[0 0.8125 1] Return Selected Stimuli if Sensed
  (bind _info (Class|AIPerceptionComponent|GetActorsPerception (Variables|Default|GetAIPerception) Actor))
  (for _array_element (.LastSensedStimuli (Utilities|Struct|BreakActorPerceptionBlueprintInfo _info))
    (bind _returnvalue (Class|AIPerceptionSystem|GetSenseClassforStimulus _array_element))
    (if (== _returnvalue (Utilities|Select :Index Sense :NewEnumerator0 "/Script/AIModule.AISense_Sight" :NewEnumerator1 "/Script/AIModule.AISense_Hearing"))
      (return (.bSuccessfullySensed (Utilities|Struct|BreakAIStimulus _array_element)) _array_element))))

(fn CanSeeTarget
  ;[0 0.8125 1] Return If Seen Actor
  (return (GameplayTags|HasTag (Variables|/Game/Blueprints/AI/BP_Enemy.BP_Enemy_C|GetTagContainer (Variables|Actors|GetRefEnemy)) "(TagName=\"Enemy.Senses.Sight\")" true)))

(fn HandleSensedSight
  (params (Actor :type Actor%20Object%20Reference) (Stimulus :type AI%20Stimulus%20Structure))
  (Utilities|Array|AddUnique (Variables|Actors|GetKnownSeenActors) Actor)
  (GameplayTags|AddGameplayTag (Variables|/Game/Blueprints/AI/BP_Enemy.BP_Enemy_C|GetTagContainer (Variables|Actors|GetRefEnemy)) "(TagName=\"Enemy.Senses.Sight\")" :!class /Script/GameplayTags.BlueprintGameplayTagLibrary)
  (if (Pure|IsEnemyChasing)
    ;[0.1719 1 0] If Was Chasing and did not forget, chase without DetectionMeter
    (Variables|Actors|SetTargetActor Actor)
    (Gameplay|StateTree|SendStateTreeEvent (Variables|Default|GetStateTreeAI) (Utilities|Struct|MakeStateTreeEvent "(TagName=\"StateTree.Chase\")" "None" "None") :!class /Script/GameplayStateTreeModule.StateTreeComponent)
    (else
      ;[0 1 0.4609] If Not Chasing Activate Detection Meter
      (bind _output_get (Variables|Actors|SetTargetActor Actor))
      (Class|BPIDetectionSystem|ActivateDetection(Message) (Variables|Actors|GetRefEnemy) _output_get))))

(fn HandleSensedHearing
  (params (Actor :type Actor%20Object%20Reference) (Stimulus :type AI%20Stimulus%20Structure))
  ;[0 1 0.2266] Set Last Heard Location and Set State As Investigation
  (Variables|Locations|SetLastHeardLocation (.StimulusLocation (Utilities|Struct|BreakAIStimulus Stimulus)))
  (Gameplay|StateTree|SendStateTreeEvent (Variables|Default|GetStateTreeAI) (Utilities|Struct|MakeStateTreeEvent "(TagName=\"StateTree.Investigation.Sound\")" "None" "None") :!class /Script/GameplayStateTreeModule.StateTreeComponent))

(fn HandleForgotActor
  (params (Actor :type Actor%20Object%20Reference))
  (bind _refenemy (Variables|Actors|GetRefEnemy))
  ;[1 0.1406 0] Clear target info when forgotten and send back to routine state.
  (Utilities|Array|RemoveItem (Variables|Actors|GetKnownSeenActors) Actor)
  (if (== Actor (Game|Player|GetPlayerPawn 0))
    (Class|BPIDetectionSystem|DisableDetection(Message) (Variables|Actors|GetRefEnemy))
    (Class|BPIDetectionWidget|OnUndetection(Message) (Variables|Actors|GetRefEnemy) 0.0)
    (Variables|Actors|SetTargetActor 0)
    (GameplayTags|RemoveGameplayTag (Variables|/Game/Blueprints/AI/BP_Enemy.BP_Enemy_C|GetTagContainer _refenemy) "(TagName=\"Enemy.Status.Chasing\")" :!class /Script/GameplayTags.BlueprintGameplayTagLibrary)
    (Variables|/Game/Blueprints/AI/BP_Enemy.BP_Enemy_C|SetDetectionMeter _refenemy 0.0)
    (Gameplay|StateTree|SendStateTreeEvent (Variables|Default|GetStateTreeAI) (Utilities|Struct|MakeStateTreeEvent "(TagName=\"StateTree.Routine\")" "None" "None") :!class /Script/GameplayStateTreeModule.StateTreeComponent)))

(fn HandleLostSight
  (params (Actor :type Actor%20Object%20Reference))
  ;[1 0.8672 0] If Target Actor Line of Sight is Lost,  Go To Seeking State
  (GameplayTags|RemoveGameplayTag (Variables|/Game/Blueprints/AI/BP_Enemy.BP_Enemy_C|GetTagContainer (Variables|Actors|GetRefEnemy)) "(TagName=\"Enemy.Senses.Sight\")" :!class /Script/GameplayTags.BlueprintGameplayTagLibrary)
  (bind _targetactor (Variables|Actors|GetTargetActor)
    (:then
      (if (Math|Boolean|ANDBoolean (== Actor _targetactor) (Pure|IsEnemyChasing) (Pure|IsEnemyFar))
        (Gameplay|StateTree|SendStateTreeEvent (Variables|Default|GetStateTreeAI) (Utilities|Struct|MakeStateTreeEvent "(TagName=\"StateTree.Seeking\")" "None" "None") :!class /Script/GameplayStateTreeModule.StateTreeComponent)))
    (:else)))

(fn SetLastSeenLocation
  ;[0.1484 0 1] Predict Target Location
  (bind _targetactor (Variables|Actors|GetTargetActor)
    (:then
      (Variables|Locations|SetLastSeenLocation (* (+ (Transformation|GetActorLocation _targetactor) (Transformation|GetVelocity _targetactor)) 1.0)))
    (:else)))

(fn GetRef
  (params (Pawn :type Actor%20Object%20Reference))
  (bind _asbp_enemy (Utilities|Casting|CastToBP_Enemy Pawn))
  (Variables|Actors|SetRefEnemy _asbp_enemy)
  (bind _asbp_core_character (Utilities|Casting|CastToBP_Core_Character (Game|Player|GetPlayerPawn 0)))
  (Variables|Actors|SetRefCoreCharacter _asbp_core_character))

(fn SetTimers
  ;[1 0.5391 0] Initialize Timers
  (bind _returnvalue (Utilities|Time|SetTimerbyEvent (EventDispatchers|CreateEvent :!event Custom|CheckIfForgottenSeenActor) 0.5 true))
  (Variables|Timers|SetCheckForgottenActorsTimer _returnvalue)
  (bind _returnvalue_2 (Utilities|Time|SetTimerbyEvent (EventDispatchers|CreateEvent :!event Custom|CheckZoneChange) 0.5 true))
  (Variables|Timers|SetCheckZoneChangeTimer _returnvalue_2))

(fn IsEnemyChasing
  (return (GameplayTags|HasTag (Variables|/Game/Blueprints/AI/BP_Enemy.BP_Enemy_C|GetTagContainer (Variables|Actors|GetRefEnemy)) "(TagName=\"Enemy.Status.Chasing\")" true)))

(fn RefreshTarget
  ;[0 0.4141 1] Refresh Target
  (Variables|Actors|SetTargetActor (Game|Player|GetPlayerPawn 0)))

(fn IsEnemyFar
  (Variables|Actors|GetTargetActor
    (:then
      (Variables|Actors|GetRefEnemy
        (:then
          (return (>= (Transformation|GetDistanceTo (Variables|Actors|GetRefEnemy) (Variables|Actors|GetTargetActor)) 1e+03)))
        (:else)))
    (:else)))