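; Patrol route actor that supplies AI with world-space waypoints along a spline.
; IncrementPatrolRoute steps PatrolIndex by Direction, then either wraps to zero or reverses for ping-pong movement, depending on ShouldLoop.
; The end check fires when the index equals the spline point count, one past the last valid index.
; GetSplinePointAsWorldPosition returns the world location of the current point.
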(event Custom|IncrementPatrolRoute
  (params (ShouldLoop :type Boolean))
  (bind _output_get (Variables|Default|SetPatrolIndex (+ (Variables|Default|GetPatrolIndex) (Variables|Default|GetDirection))))
  (if (== _output_get (- (Spline|GetNumberOfSplinePoints (Variables|Default|GetSpline)) 0))
    (if ShouldLoop
      (Variables|Default|SetPatrolIndex 0)
      (else
        (Variables|Default|SetDirection -1)))
    (elif (== (Variables|Default|GetPatrolIndex) 0)
      (Variables|Default|SetDirection 1))))

(fn ConstructionScript)

(fn GetSplinePointasWorldPosition
  (return (Spline|GetLocationatSplinePoint (Variables|Default|GetSpline) (Variables|Default|GetPatrolIndex) "World")))