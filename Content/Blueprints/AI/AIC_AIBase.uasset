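; AI controller for BP_AIBase pawns that restarts its StateTree a tick after possession and turns perception of the player into behavior events.
; Sight depends on AI type and the player's zone: guards chase in Private or Secure zones and clear their target in Public, while the Civilian branch is empty.
; Hearing stores the sound location and sends a sound investigation event for any AI type.
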(event OnTargetPerceptionUpdated(AIPerception)
  (params (Actor :type Actor%20Object%20Reference) (Stimulus :type AI%20Stimulus%20Structure))
  (if (== Actor (Game|GetPlayerCharacter 0))
    (Utilities|FlowControl|Sequence
      (:then_0
        (bind (_sensed _stimulus) (CallFunction|CanSenseActor Actor "NewEnumerator0"))
        (if _sensed
          (CallFunction|HandleSensedSight Actor _stimulus)))
      (:then_1
        (bind (_sensed_2 _stimulus_2) (CallFunction|CanSenseActor Actor "NewEnumerator1"))
        (if _sensed_2
          (CallFunction|HandleSensedHearing Actor _stimulus_2))))))

(event EventPossess
  (params (PossessedPawn :type Pawn%20Object%20Reference))
  (Utilities|FlowControl|DelayUntilNextTick)
  (Class|BrainComponent|RestartLogic (Variables|Default|GetStateTreeAI))
  (CallFunction|GetAIBaseRef PossessedPawn))

(fn ConstructionScript)

(fn GetAIBaseRef
  (params (Pawn :type Actor%20Object%20Reference))
  (bind _asbp_aibase (Utilities|Casting|CastToBP_AIBase Pawn))
  (Variables|Default|SetRefAIBase _asbp_aibase))

(fn CanSenseActor
  (params (Actor :type Actor%20Object%20Reference) (Sense :type E_AISense%20Enum :default "NewEnumerator0"))
  (bind _info (Class|AIPerceptionComponent|GetActorsPerception (Variables|Default|GetAIPerception) Actor))
  (for _array_element (.LastSensedStimuli (Utilities|Struct|BreakActorPerceptionBlueprintInfo _info))
    (bind _returnvalue (Class|AIPerceptionSystem|GetSenseClassforStimulus _array_element))
    (if (== _returnvalue (Utilities|Select :Index Sense :NewEnumerator0 "/Script/AIModule.AISense_Sight" :NewEnumerator1 "/Script/AIModule.AISense_Hearing"))
      (return (.bSuccessfullySensed (Utilities|Struct|BreakAIStimulus _array_element)) _array_element))))

(fn HandleSensedSight
  (params (Actor :type Actor%20Object%20Reference) (Stimulus :type AI%20Stimulus%20Structure))
  (switch Utilities|FlowControl|Switch|SwitchonE_AIType (Variables|/Game/Blueprints/AI/BP_AIBase.BP_AIBase_C|GetAIType (Variables|Default|GetRefAIBase))
    (:NewEnumerator0
      (bind _zonetype (Class|BPIZoneDetector|GetCurrentZone(Message) Actor))
      (switch Utilities|FlowControl|Switch|SwitchonE_ZoneType _zonetype
        (:NewEnumerator0
          (Variables|Default|SetTargetActor 0))
        (:NewEnumerator1
          (Variables|Default|SetTargetActor Actor :!label _label)
          (Gameplay|StateTree|SendStateTreeEvent (Variables|Default|GetStateTreeAI) (Utilities|Struct|MakeStateTreeEvent "(TagName=\"StateTree.Chase\")" "None" "None") :!class /Script/GameplayStateTreeModule.StateTreeComponent))
        (:NewEnumerator2
          (goto _label))))
    (:NewEnumerator1
      (bind _zonetype_2 (Class|BPIZoneDetector|GetCurrentZone(Message) Actor))
      (switch Utilities|FlowControl|Switch|SwitchonE_ZoneType _zonetype_2))))

(fn HandleSensedHearing
  (params (Actor :type Actor%20Object%20Reference) (Stimulus :type AI%20Stimulus%20Structure))
  (Variables|Default|SetLastHeardLocation (.StimulusLocation (Utilities|Struct|BreakAIStimulus Stimulus)))
  (Gameplay|StateTree|SendStateTreeEvent (Variables|Default|GetStateTreeAI) (Utilities|Struct|MakeStateTreeEvent "(TagName=\"StateTree.Investigation.Sound\")" "None" "None") :!class /Script/GameplayStateTreeModule.StateTreeComponent))