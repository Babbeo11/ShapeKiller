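; BP_AIBase is a base Blueprint for AI that holds an AI type, a current zone type and a list of idle points.
; On BeginPlay it caches the location of the current idle point.
; Each call to GetIdlePointLocation that finds a valid point stores its location and advances the index, wrapping to cycle through the list.
; Simple accessor functions expose the AI type and read or set the current zone.
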(event EventBeginPlay
  (CallFunction|GetIdlePointLocation))

(fn ConstructionScript)

(fn GetIdlePointLocation
  (Utilities|IsValid (Utilities|Array|Get(acopy) (Variables|PathSettings|GetIdlePoints) (Variables|Default|GetIndex))
    (:Is%20Valid
      (Variables|Default|SetIdlePointLocation (Transformation|GetActorLocation (Utilities|Array|Get(acopy) (Variables|PathSettings|GetIdlePoints) (Variables|Default|GetIndex))))
      (Math|Integer|IncrementInt (Variables|Default|GetIndex)
        (:%20%20
          (if (>= (Variables|Default|GetIndex) (Utilities|Array|Length (Variables|PathSettings|GetIdlePoints)))
            (Variables|Default|SetIndex 0)))))))

(fn GetAIType
  (return (Variables|AISettings|GetAIType)))

(fn GetCurrentZone
  (return (Variables|Default|GetCurrentZoneType)))

(fn SetCurrentZone
  (params (ZoneType :type E_ZoneType%20Enum :default "NewEnumerator0"))
  (Variables|Default|SetCurrentZoneType ZoneType)
  (return true))