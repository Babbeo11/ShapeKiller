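; Detection system component that raises or lowers an enemy's detection meter against a target and notifies the player pawn of changes.
; A looping timer, unpaused by ActivateDetection, evaluates non-chasing enemies and pauses once the meter fills.
; The meter rises when the enemy has sight and player tags match the target's Public or Private zone rules.
; Distance scales the whole adjusted meter, and zone-flagged sprinting increases the gain; Secure zones have no criteria branch.
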(event EventBeginPlay
  (bind _returnvalue (Utilities|Time|SetTimerbyEvent (EventDispatchers|CreateEvent :!event HandleDetection) 0.1 true))
  (bind _output_get (Variables|Default|SetHandleDetectionTimer _returnvalue))
  (Utilities|Time|PauseTimerbyHandle _output_get)
  (bind _asbp_core_character (Utilities|Casting|CastToBP_Core_Character (Game|GetPlayerCharacter 0)))
  (Variables|Default|SetRefCoreCharacter _asbp_core_character))

(event EventEndPlay
  (params (EndPlayReason :type EEndPlayReason%20Enum :default "Destroyed"))
  (Utilities|Time|ClearandInvalidateTimerbyHandle (Variables|Default|GetHandleDetectionTimer)))

(fn ActivateDetection
  (params (TargetActor :type Actor%20Object%20Reference) (EnemyActor :type BP%20Enemy%20Object%20Reference))
  (CallFunction|SetInfo TargetActor EnemyActor)
  (Utilities|Time|UnpauseTimerbyHandle (Variables|Default|GetHandleDetectionTimer))
  (return))

(fn SetInfo
  (params (TargetActor :type Actor%20Object%20Reference) (EnemyActor :type BP%20Enemy%20Object%20Reference))
  (Utilities|IsValid TargetActor
    (:Is%20Valid
      (bind _output_get (Variables|Default|SetTargetActor TargetActor))
      (bind _detectionparameters (Class|BPIDetectionSystem|GetDetectionParameters(Message) _output_get))
      (Variables|Default|SetDetectionParameters _detectionparameters)
      (Utilities|IsValid EnemyActor
        (:Is%20Valid
          (Variables|Default|SetEnemyActor EnemyActor))))))

(fn HandleDetection
  (bind _returnvalue (Game|Player|GetPlayerPawn 0))
  (if (not (Pure|IsEnemyChasing))
    (if (Math|Float|InRange(Float) (Variables|/Game/Blueprints/AI/BP_Enemy.BP_Enemy_C|GetDetectionMeter (Variables|Default|GetEnemyActor)) 0.0 1e+02 true false)
      (if (Pure|IsEnemySeeing)
        (Utilities|DetectCriteria
          (:Detect
            (bind _detectionlevel (CallFunction|IncrementDetectionLevel))
            (Class|BPIDetectionSystem|OnDetection(Message) (Game|Player|GetPlayerPawn 0) (Variables|Default|GetEnemyActor) _detectionlevel))
          (:Undetect
            (bind _detectionlevel_2 (CallFunction|DecrementDetectionLevel :!label _label))
            (Class|BPIDetectionSystem|OnUndetection(Message) _returnvalue _detectionlevel_2)
            (Class|BPIDetectionSystem|OnDetectionZero(Message) _returnvalue _detectionlevel_2)))
        (else
          (goto _label)))
      (elif (>= (Variables|/Game/Blueprints/AI/BP_Enemy.BP_Enemy_C|GetDetectionMeter (Variables|Default|GetEnemyActor)) 1e+02)
        (Utilities|Time|PauseTimerbyHandle (Variables|Default|GetHandleDetectionTimer))))))

(fn DisableDetection
  (Utilities|Time|PauseTimerbyHandle (Variables|Default|GetHandleDetectionTimer))
  (return))

(fn IncrementDetectionLevel
  (bind _enemyactor (Variables|Default|GetEnemyActor))
  (bind _enemyactor_2 (Variables|Default|GetEnemyActor))
  (bind _targetactor (Variables|Default|GetTargetActor))
  (bind _enemyactor_3 (Variables|Default|GetEnemyActor))
  (bind _detectionparameters (Variables|Default|GetDetectionParameters))
  (bind _returnvalue (Transformation|GetDistanceTo _targetactor _enemyactor_3))
  (bind _returnvalue_2 (Math|Float|MapRangeClamped _returnvalue 1.5e+02 8e+02 1.2 0.8))
  (bind _zonetype (Class|BPIPlayerInfo|GetCurrentZone(Message) (Variables|Default|GetTargetActor)))
  (if (Pure|HasSprintingTag (Utilities|Select :Index _zonetype :NewEnumerator0 (Variables|/Game/Blueprints/DataAssets/DetectionParameters/DetectionParameters.DetectionParameters_C|GetPublicTag _detectionparameters) :NewEnumerator1 (Variables|/Game/Blueprints/DataAssets/DetectionParameters/DetectionParameters.DetectionParameters_C|GetPrivateTag _detectionparameters) :NewEnumerator2 ""))
    (bind _output_get (LocalVariables|SetSum 15.0))
    (bind _output_get_2 (Variables|/Game/Blueprints/AI/BP_Enemy.BP_Enemy_C|SetDetectionMeter _enemyactor (* (+ (Variables|/Game/Blueprints/AI/BP_Enemy.BP_Enemy_C|GetDetectionMeter _enemyactor) _output_get) _returnvalue_2)))
    (return _output_get_2)
    (else
      (bind _output_get_3 (LocalVariables|SetSum 1e+01))
      (bind _output_get_4 (Variables|/Game/Blueprints/AI/BP_Enemy.BP_Enemy_C|SetDetectionMeter _enemyactor_2 (* (+ (Variables|/Game/Blueprints/AI/BP_Enemy.BP_Enemy_C|GetDetectionMeter _enemyactor_2) _output_get_3) _returnvalue_2)))
      (return _output_get_4))))

(fn IsEnemyChasing
  (bind _enemytag (Class|BPIDetectionSystem|GetTag(Message) (Variables|Default|GetEnemyActor)))
  (return (GameplayTags|HasTag _enemytag "(TagName=\"Enemy.Status.Chasing\")" true)))

(fn IsEnemySeeing
  (return (GameplayTags|HasTag (Variables|/Game/Blueprints/AI/BP_Enemy.BP_Enemy_C|GetTagContainer (Variables|Default|GetEnemyActor)) "(TagName=\"Enemy.Senses.Sight\")" true)))

(fn HasSprintingTag
  (params (TagContainer :type Gameplay%20Tag%20Container%20Structure%20%28by%20ref%29))
  (return (and (GameplayTags|HasTag (Variables|/Game/Blueprints/Gamemode/Core/BP_Core_Character.BP_Core_Character_C|GetTagsContainer (Variables|Default|GetRefCoreCharacter)) "(TagName=\"Player.Movement.Sprinting\")" true) (GameplayTags|HasTag TagContainer "(TagName=\"Player.Movement.Sprinting\")" true))))

(fn DecrementDetectionLevel
  (bind _enemyactor (Variables|Default|GetEnemyActor))
  (if (>= (* (- (Variables|/Game/Blueprints/AI/BP_Enemy.BP_Enemy_C|GetDetectionMeter _enemyactor) 1e+01) (Math|Float|MapRangeClamped (Transformation|GetDistanceTo (Variables|Default|GetTargetActor) (Variables|Default|GetEnemyActor)) 1.5e+02 8e+02 0.8 1.2)) 0.0)
    (bind _output_get (Variables|/Game/Blueprints/AI/BP_Enemy.BP_Enemy_C|SetDetectionMeter _enemyactor (* (- (Variables|/Game/Blueprints/AI/BP_Enemy.BP_Enemy_C|GetDetectionMeter _enemyactor) 1e+01) (Math|Float|MapRangeClamped (Transformation|GetDistanceTo (Variables|Default|GetTargetActor) (Variables|Default|GetEnemyActor)) 1.5e+02 8e+02 0.8 1.2))))
    (else
      (Variables|/Game/Blueprints/AI/BP_Enemy.BP_Enemy_C|SetDetectionMeter _enemyactor 0.0)))
  (return _output_get))