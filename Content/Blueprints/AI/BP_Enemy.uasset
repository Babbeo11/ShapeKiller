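; BP_Enemy is an AI enemy actor with player detection, idle points, timed status effects and ragdoll death.
; It forwards detection calls to BPCDetectionSystem, while detection events use a reversible Timeline to drive an on-screen detection meter widget.
; BPC_EnemyStatus events add gameplay tags for a set duration and, on death, stop ticking, enable physics and collapse the meter.
; GetIdlePointLocation cycles through IdlePoints, supplying a location on each call.
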(event OnStatusChange(BPC_EnemyStatus)
  (params (StatusTag :type Gameplay%20Tag%20Structure) (StatusDuration :type Float%20%28double-precision%29))
  (bind _tagcontainer (Variables|EnemyInfo|GetTagContainer))
  (GameplayTags|AddGameplayTag _tagcontainer StatusTag :!class /Script/GameplayTags.BlueprintGameplayTagLibrary)
  (Utilities|FlowControl|Delay StatusDuration)
  (GameplayTags|RemoveGameplayTag _tagcontainer StatusTag :!class /Script/GameplayTags.BlueprintGameplayTagLibrary))

(event OnDeath(BPC_EnemyStatus)
  (Actor|Tick|SetActorTickEnabled false)
  (Class|SkeletalMeshComponent|SetAllBodiesSimulatePhysics (Variables|Character|GetMesh) true)
  (Widget|SetVisibility (Variables|DetectionMeter|GetDetectionMeterWidget) "Collapsed"))

(event EventBeginPlay
  (CallFunction|GetIdlePointLocation)
  (bind _returnvalue (UserInterface|CreateWidget "/Game/Blueprints/UI/WB_DetectionMeter.WB_DetectionMeter_C" (Game|GetPlayerController 0)))
  (Variables|DetectionMeter|SetDetectionMeterWidget _returnvalue))

(event EventOnDetection
  (params (DetectionMeter :type Float%20%28double-precision%29))
  (bind _detectionmeterwidget (Variables|DetectionMeter|GetDetectionMeterWidget))
  (bind _progressbar (Variables|/Game/Blueprints/UI/WB_DetectionMeter.WB_DetectionMeter_C|GetProgressBar _detectionmeterwidget))
  ;[0.1719 1 0] DetectionMeterWidget
  (UserInterface|Viewport|AddtoViewport (Variables|DetectionMeter|GetDetectionMeterWidget) 0)
  (Variables|/Game/Blueprints/UI/WB_DetectionMeter.WB_DetectionMeter_C|SetEnemy (Variables|DetectionMeter|GetDetectionMeterWidget) self)
  (Widget|SetVisibility _progressbar "Visible")
  (bind (_direction _detection) (Timeline|Timeline Play)
    (:Update
      (Progress|SetPercent _progressbar (Math|Float|MapRangeClamped (Math|Float|Lerp 0.0 (Utilities|Select :Index _direction :Forward DetectionMeter :Backward (stale EventOnUndetection DetectionMeter)) _detection) 0.0 1e+02 0.0 1.0)))))

(event EventOnUndetection
  (params (DetectionMeter :type Float%20%28double-precision%29))
  (bind _detectionmeterwidget (Variables|DetectionMeter|GetDetectionMeterWidget))
  (bind _progressbar (Variables|/Game/Blueprints/UI/WB_DetectionMeter.WB_DetectionMeter_C|GetProgressBar _detectionmeterwidget))
  ;[0.1719 1 0] DetectionMeterWidget
  (if (> DetectionMeter 0.0)
    (bind (_direction _detection) (Timeline|Timeline Reverse)
      (:Update
        (Progress|SetPercent (Variables|/Game/Blueprints/UI/WB_DetectionMeter.WB_DetectionMeter_C|GetProgressBar (Variables|DetectionMeter|GetDetectionMeterWidget)) (Math|Float|MapRangeClamped (Math|Float|Lerp 0.0 (Utilities|Select :Index _direction :Forward (stale EventOnDetection DetectionMeter) :Backward DetectionMeter) _detection) 0.0 1e+02 0.0 1.0))))
    (else
      (Widget|SetVisibility _progressbar "Hidden")
      (Progress|SetPercent _progressbar 0.0)
      (Widget|RemovefromParent (Variables|DetectionMeter|GetDetectionMeterWidget)))))

(event EventDestroyed
  (bind _detectionmeterwidget (Variables|DetectionMeter|GetDetectionMeterWidget)
    (:then
      (Widget|RemovefromParent _detectionmeterwidget))
    (:else)))

(fn ConstructionScript)

(fn GetIdlePointLocation
  (Utilities|IsValid (Utilities|Array|Get(acopy) (Variables|PathSettings|GetIdlePoints) (Variables|Default|GetIndex))
    (:Is%20Valid
      (Variables|EnemyInfo|SetIdlePointLocation (Transformation|GetActorLocation (Utilities|Array|Get(acopy) (Variables|PathSettings|GetIdlePoints) (Variables|Default|GetIndex))))
      (Math|Integer|IncrementInt (Variables|Default|GetIndex)
        (:%20%20
          (if (>= (Variables|Default|GetIndex) (Utilities|Array|Length (Variables|PathSettings|GetIdlePoints)))
            (Variables|Default|SetIndex 0)))))))

(fn CheckDetectionMeter
  (if (>= (Variables|DetectionMeter|GetDetectionMeter) 1e+02)
    (Default|CallOnDetectedEnemy)))

(fn ActivateDetection
  (params (TargetActor :type Actor%20Object%20Reference))
  (Default|ActivateDetection (Variables|Default|GetBPC_DetectionSystem) TargetActor self)
  (return true))

(fn DisableDetection
  (Default|DisableDetection (Variables|Default|GetBPC_DetectionSystem))
  (return true))

(fn GetDetectionParameters
  (return 0))

(fn GetTag
  (return (Variables|EnemyInfo|GetTagContainer)))