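; BP_Radio is a radio distraction Blueprint whose logic is currently inactive.
; Its UseAbility event is empty, and both graphs hold unconnected logic that never runs.
; That leftover logic checks for the player pawn and, in a Private zone, reports a noise event at the box or actor location with the player as instigator.
; The construction script only calls its parent.
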(event EventUseAbility)

(fn ConstructionScript
  (|CallParentFunction))