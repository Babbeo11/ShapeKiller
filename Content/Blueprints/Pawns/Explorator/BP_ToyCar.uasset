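; Physics-driven toy car pawn that drives along the control rotation's yaw, with a separate modifier for reversing.
; Move applies acceleration to the static mesh and clamps its velocity to walk or sprint speed, chosen by the core character's sprint tag.
; The same event consumes the character's stamina and turns the mesh toward the aim yaw by a clamped, proportional step that handles the 180-degree wrap.
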(event EventTick
  (params (DeltaSeconds :type Float%20%28single-precision%29))
  (|CallParentFunction DeltaSeconds))

(event EventBeginPlay
  (|CallParentFunction))

(event EventMove
  (params (XAxis :type Float%20%28double-precision%29) (YAxis :type Float%20%28double-precision%29))
  (bind _reftocorecharacter (Variables|Default|GetRefToCoreCharacter))
  (bind _staticmesh (Variables|Default|GetStaticMesh))
  (bind _bpc_status (Variables|/Game/Blueprints/Gamemode/Core/BP_Core_Character.BP_Core_Character_C|GetBPC_Status _reftocorecharacter))
  ;[0.15 0.15 0.15 0.5] Move the pawn using physics
  (Physics|AddForce _staticmesh (* (Math|Vector|GetForwardVector (Math|Rotator|MakeRotator 0.0 0.0 (.yaw (Pawn|GetControlRotation :!class /Script/Engine.Pawn)))) YAxis (Variables|Default|GetMovementModifier) (Math|Float|SelectFloat (Variables|Default|GetReverseMovementModifier) 1.0 (< YAxis 0.0))) "None" true)
  (bind _returnvalue (Physics|GetPhysicsLinearVelocity _staticmesh "None"))
  (Physics|SetPhysicsLinearVelocity _staticmesh (Math|Vector|ClampVectorSize _returnvalue 0.0 (* (Math|Float|SelectFloat (Variables|Default|GetSprintMovementSpeed) (Variables|Default|GetWalkMovementSpeed) (GameplayTags|HasTag (Variables|/Game/Blueprints/Gamemode/Core/BP_Core_Character.BP_Core_Character_C|GetTagsContainer (Variables|Default|GetRefToCoreCharacter)) "(TagName=\"Player.Movement.Sprinting\")")) (Variables|Default|GetMovementModifier))) false "None")
  ;;[0.15 0.15 0.15 0.5] Adjust mesh rotation to match controller rotation
  (Default|ConsumeStamina _bpc_status (Variables|Default|GetWalkStaminaModifier) (Variables|/Game/Blueprints/Components/BPC_PlayerStatus.BPC_PlayerStatus_C|GetStaminaConsumeStep _bpc_status))
  (bind _yawoffset (CallFunction|CalculateYawOffset))
  (Transformation|AddWorldRotation (Variables|Default|GetStaticMesh) (Math|Rotator|MakeRotator 0.0 0.0 _yawoffset) false false))

(fn ConstructionScript
  (|CallParentFunction))

(fn CalculateYawOffset
  (bind _returnvalue (Pawn|GetBaseAimRotation))
  (bind _staticmesh (Variables|Default|GetStaticMesh))
  (bind _returnvalue_2 (Transformation|GetWorldRotation _staticmesh))
  (bind _returnvalue_3 (- (.yaw _returnvalue_2) (.yaw _returnvalue)))
  (bind _returnvalue_4 (Math|Float|Absolute(Float) _returnvalue_3))
  (return (* (Math|Float|Clamp(Float) _returnvalue_4 0.0 2e+01) (Math|Float|SelectFloat -0.2 0.2 (> (.yaw _returnvalue_2) (.yaw _returnvalue))) (Math|Float|SelectFloat -1.0 1.0 (> _returnvalue_4 1.8e+02)))))