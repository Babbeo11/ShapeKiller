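; Extinguisher Blueprint whose ability spends charge to apply a timed status effect to whatever it hits.
; UseAbility clamps the reduced charge at zero, prints it as debug text, then runs CheckAbilityHits.
; That box-traces from the mesh's EmissionSocket toward a camera-forward point at ability range, with debug drawing.
; Each hit actor's first BPI_Status component receives the effect and duration through ApplyStatusMessage.
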(event EventBeginPlay
  (|CallParentFunction))

(event EventUseAbility
  (if (> (Variables|Ability|GetAbilityCharge) 0.0)
    (Variables|Ability|SetAbilityCharge (Math|Float|SelectFloat (- (Variables|Ability|GetAbilityCharge) (Variables|Ability|GetAbilityChargeConsume)) 0.0 (< 0.0 (- (Variables|Ability|GetAbilityCharge) (Variables|Ability|GetAbilityChargeConsume)))))
    (Development|PrintString (Utilities|String|Append "REMAINING CHARGE: " (Utilities|String|ToString(Float) (Math|Float|SelectFloat (- (Variables|Ability|GetAbilityCharge) (Variables|Ability|GetAbilityChargeConsume)) 0.0 (< 0.0 (- (Variables|Ability|GetAbilityCharge) (Variables|Ability|GetAbilityChargeConsume)))))) true true "(R=0.000000,G=0.660000,B=1.000000,A=1.000000)" 0.05)
    (bind (_outhits _hit_) (CallFunction|CheckAbilityHits))
    (if _hit_
      (for _array_element _outhits
        (if (Utilities|Array|IsNotEmpty (Class|Actor|GetComponentsbyInterface (.HitActor (Collision|BreakHitResult _array_element)) "/Game/Blueprints/Interfaces/BPI_Status.BPI_Status_C"))
          (bind _array_element_2 (Utilities|Array|ForEachLoopwithBreak (Class|Actor|GetComponentsbyInterface (.HitActor (Collision|BreakHitResult _array_element)) "/Game/Blueprints/Interfaces/BPI_Status.BPI_Status_C") :!label _label)
            (:LoopBody
              (Class|BPIStatus|ApplyStatus(Message) _array_element_2 (Variables|Ability|GetAbilityEffect) (Variables|Ability|GetAbilityEffectDuration))
              (goto _label Break))))))))

(fn ConstructionScript
  (|CallParentFunction))

(fn CheckAbilityHits
  (bind _tpcamera (Variables|Default|GetTPCamera))
  (bind _staticmesh (Variables|Default|GetStaticMesh))
  (bind _returnvalue (Transformation|GetSocketLocation _staticmesh "EmissionSocket"))
  (bind _outhits (Class|KismetSystemLibrary|BoxTraceMulti _returnvalue (+ _returnvalue (- (+ (Transformation|GetWorldLocation _tpcamera) (* (Math|Vector|GetForwardVector _tpcamera) (Variables|Ability|GetAbilityRange))) _returnvalue)) "30.000000,30.000000,30.000000" "0, 0, 0" "TraceTypeQuery5" false 0 "ForDuration" true "(R=1.000000,G=0.000000,B=0.000000,A=1.000000)" "(R=0.000000,G=1.000000,B=0.000000,A=1.000000)" 0.05))
  (return _outhits (Utilities|Array|IsNotEmpty _outhits)))