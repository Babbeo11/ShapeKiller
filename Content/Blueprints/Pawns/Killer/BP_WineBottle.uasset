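; BP_WineBottle is a Killer pawn whose ability shoots its cork.
; UseAbility spawns a BP_Cork actor at the Cork component, owned and instigated by the bottle.
; The shot is rotated toward a point CorkPrecisionRange ahead of the third-person camera, so it follows the camera's aim.
; It then clears HasCork and prints a message, but the HasCork check and Cork component removal are disconnected, so neither runs.
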(event EventBeginPlay
  (|CallParentFunction))

(event EventTick
  (params (DeltaSeconds :type Float%20%28single-precision%29))
  (|CallParentFunction DeltaSeconds))

(event EventUseAbility
  (bind _self self)
  (bind _cork (Variables|Default|GetCork))
  (bind _tpcamera (Variables|Default|GetTPCamera))
  (bind _returnvalue (Transformation|GetWorldLocation _cork))
  (Game|SpawnActorfromClass "/Game/Blueprints/Pawns/Killer/BP_Cork.BP_Cork_C" (Math|Transform|MakeTransform _returnvalue (Math|Rotator|FindLookatRotation _returnvalue (+ (Transformation|GetWorldLocation _tpcamera) (* (Math|Vector|GetForwardVector _tpcamera) (Variables|Default|GetCorkPrecisionRange)))) "1.000000,1.000000,1.000000") "AlwaysSpawn" "MultiplyWithRoot" _self _self)
  (Variables|Default|SetHasCork? false)
  (Development|PrintString "Cork has been shot!"))

(fn ConstructionScript
  (|CallParentFunction))