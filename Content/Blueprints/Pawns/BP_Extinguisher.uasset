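; BP_Extinguisher is a pawn Blueprint with a use-ability event, built on a parent that it calls on begin play and construction.
; UseAbility runs an invisible box trace on the Visibility channel from the third-person camera along its forward vector, out to AbilityRange.
; The trace result is unused, so the ability has no effect in this graph yet.
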(event EventBeginPlay
  (|CallParentFunction))

(event EventUseAbility
  (bind _tpcamera (Variables|Default|GetTPCamera))
  (bind _returnvalue (Transformation|GetWorldLocation _tpcamera))
  (Collision|BoxTraceByChannel _returnvalue (+ _returnvalue (* (Math|Vector|GetForwardVector _tpcamera) (Variables|Ability|GetAbilityRange))) "50.000000,50.000000,50.000000" "0, 0, 0" "TraceTypeQuery1" false 0 "None"))

(fn ConstructionScript
  (|CallParentFunction))