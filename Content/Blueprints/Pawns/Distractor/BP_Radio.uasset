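; Radio distractor that the player toggles on and off through interaction to emit noise for AI hearing.
; A FlipFlop starts or clears a looping half-second timer, which presumably drives EmitSound.
; EmitSound reports a "Radio"-tagged noise at its location with the player pawn as instigator, draining charge until the timer stops at zero.
; The character's zone check currently has empty branches, and depletion leaves IsEmitting set.
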(event EventInteraction
  (CallFunction|UseAbility))

(event Custom|EmitSound
  (bind _zonetype (Class|BPIPlayerInfo|GetCurrentZone(Message) (Variables|Default|GetRefToCoreCharacter)))
  (switch Utilities|FlowControl|Switch|SwitchonE_ZoneType _zonetype
    (:NewEnumerator0
      _)
    (:NewEnumerator1
      _))
  (Class|AISenseHearing|ReportNoiseEvent (Transformation|GetActorLocation) 1.0 (Game|Player|GetPlayerPawn 0) 0.0 "Radio")
  (bind _output_get (Variables|Default|SetAbilityCharge (Math|Float|SelectFloat (- (Variables|Default|GetAbilityCharge) (Variables|Default|GetAbilityChargeConsume)) 0.0 (> (- (Variables|Default|GetAbilityCharge) (Variables|Default|GetAbilityChargeConsume)) 0.0))))
  (Development|PrintString (Utilities|String|Append "EMITTER CHARGE: " (Utilities|String|ToString(Float) _output_get)) true true "(R=0.000000,G=0.660000,B=1.000000,A=1.000000)" 0.5)
  (if (== _output_get 0.0)
    (Utilities|Time|ClearandInvalidateTimerbyHandle (Variables|Default|GetTimerHandle))))

(event EventUseAbility
  (Utilities|FlowControl|FlipFlop
    (:A
      (if (not (Variables|Default|GetIsEmitting))
        (Variables|Default|SetIsEmitting true)
        (bind _returnvalue (Utilities|Time|SetTimerbyEvent (EventDispatchers|CreateEvent :!event Custom|EmitSound) 0.5 true true))
        (Variables|Default|SetTimerHandle _returnvalue)
        (Development|PrintString "RADIO TURNED ON")))
    (:B
      (Variables|Default|SetIsEmitting false)
      (Utilities|Time|ClearandInvalidateTimerbyHandle (Variables|Default|GetTimerHandle))
      (Development|PrintString "RADIO TURNED OFF"))))

(fn ConstructionScript
  (|CallParentFunction))