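; BP_TriggerManager is an actor that handles level trigger boxes for moving the player between floor and attic and for ending the game.
; Overlapping a stairs or elevator box with a Player-tagged actor waits TransitionTime, then teleports it to the paired box.
; Teleport offsets the player along the destination's forward vector by TeleportRange and adopts its rotation.
; The entrance box quits the game after a short delay once IsBossDead is set.
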(event OnActorBeginOverlap(EntranceBox)
  (params (OverlappedActor :type Actor%20Object%20Reference) (OtherActor :type Actor%20Object%20Reference))
  (if (Actor|ActorHasTag OtherActor "Player")
    (if (Variables|Default|GetIsBossDead?)
      (Utilities|FlowControl|Delay 3.0)
      (Game|QuitGame 0 "Quit" false))))

(event OnActorBeginOverlap(FloorStairsBox)
  (params (OverlappedActor :type Actor%20Object%20Reference) (OtherActor :type Actor%20Object%20Reference))
  (if (Actor|ActorHasTag OtherActor "Player")
    (Utilities|FlowControl|Delay (Variables|Default|GetTransitionTime))
    (CallFunction|Teleport OtherActor (Variables|Default|GetAtticStairsBox))))

(event OnActorBeginOverlap(AtticStairsBox)
  (params (OverlappedActor :type Actor%20Object%20Reference) (OtherActor :type Actor%20Object%20Reference))
  (if (Actor|ActorHasTag OtherActor "Player")
    (Utilities|FlowControl|Delay (Variables|Default|GetTransitionTime))
    (CallFunction|Teleport OtherActor (Variables|Default|GetFloorStairsBox))))

(event OnActorBeginOverlap(FloorElevatorBox)
  (params (OverlappedActor :type Actor%20Object%20Reference) (OtherActor :type Actor%20Object%20Reference))
  (if (Actor|ActorHasTag OtherActor "Player")
    (Utilities|FlowControl|Delay (Variables|Default|GetTransitionTime))
    (CallFunction|Teleport OtherActor (Variables|Default|GetAtticElevatorBox))))

(event OnActorBeginOverlap(AtticElevatorBox)
  (params (OverlappedActor :type Actor%20Object%20Reference) (OtherActor :type Actor%20Object%20Reference))
  (if (Actor|ActorHasTag OtherActor "Player")
    (Utilities|FlowControl|Delay (Variables|Default|GetTransitionTime))
    (CallFunction|Teleport OtherActor (Variables|Default|GetFloorElevatorBox))))

(fn ConstructionScript)

(fn Teleport
  (params (ActorToTeleport :type Actor%20Object%20Reference) (DestinationActor :type Actor%20Object%20Reference))
  (bind _returnvalue (Transformation|GetActorTransform DestinationActor))
  (Transformation|SetActorLocationAndRotation ActorToTeleport (+ (.location _returnvalue) (* (Transformation|GetActorForwardVector DestinationActor) (Variables|Default|GetTeleportRange))) (.rotation _returnvalue) false true))