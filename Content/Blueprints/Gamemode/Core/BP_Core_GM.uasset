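; Core game mode that owns the on-screen enemy detection meter, creating its widget for the first player at BeginPlay.
; OnDetection hands the enemy to the widget, shows the progress bar and plays a timeline that scales the meter value into the bar's percent.
; OnUndetection reverses that timeline while the passed meter is above zero, otherwise it hides and empties the bar.
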(event EventBeginPlay
  (bind _returnvalue (UserInterface|CreateWidget "/Game/Blueprints/UI/WB_DetectionMeter.WB_DetectionMeter_C" (Game|GetPlayerController 0)))
  (bind _output_get (Variables|Default|SetDetectionMeterWidget _returnvalue))
  (UserInterface|Viewport|AddtoViewport _output_get 0))

(event EventOnDetection
  (params (EnemyActor :type BP%20Enemy%20Object%20Reference) (DetectionMeter :type Float%20%28double-precision%29))
  (bind _detectionmeterwidget (Variables|Default|GetDetectionMeterWidget))
  (bind _progressbar (Variables|/Game/Blueprints/UI/WB_DetectionMeter.WB_DetectionMeter_C|GetProgressBar _detectionmeterwidget))
  ;[0.1719 1 0] DetectionMeterWidget
  (Variables|/Game/Blueprints/UI/WB_DetectionMeter.WB_DetectionMeter_C|SetEnemy (Variables|Default|GetDetectionMeterWidget) EnemyActor)
  (Widget|SetVisibility _progressbar "Visible")
  (bind (_direction _detection) (Timeline|Timeline Play)
    (:Update
      (Progress|SetPercent _progressbar (Math|Float|MapRangeClamped (Math|Float|Lerp 0.0 (Utilities|Select :Index _direction :Forward DetectionMeter :Backward (stale EventOnUndetection DetectionMeter)) _detection) 0.0 1e+02 0.0 1.0)))))

(event EventOnUndetection
  (params (DetectionMeter :type Float%20%28double-precision%29))
  (bind _detectionmeterwidget (Variables|Default|GetDetectionMeterWidget))
  (bind _progressbar (Variables|/Game/Blueprints/UI/WB_DetectionMeter.WB_DetectionMeter_C|GetProgressBar _detectionmeterwidget))
  ;[0.1719 1 0] DetectionMeterWidget
  (if (> DetectionMeter 0.0)
    (bind (_direction _detection) (Timeline|Timeline Reverse)
      (:Update
        (Progress|SetPercent (Variables|/Game/Blueprints/UI/WB_DetectionMeter.WB_DetectionMeter_C|GetProgressBar (Variables|Default|GetDetectionMeterWidget)) (Math|Float|MapRangeClamped (Math|Float|Lerp 0.0 (Utilities|Select :Index _direction :Forward (stale EventOnDetection DetectionMeter) :Backward DetectionMeter) _detection) 0.0 1e+02 0.0 1.0))))
    (else
      (Widget|SetVisibility _progressbar "Hidden")
      (Progress|SetPercent _progressbar 0.0))))

(fn ConstructionScript)