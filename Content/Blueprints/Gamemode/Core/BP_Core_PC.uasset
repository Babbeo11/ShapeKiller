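; Core player controller that routes Enhanced Input to the player character or the object it is possessing.
; On BeginPlay it caches the BP_Core_Character reference and adds the default mapping context.
; Move, look and jump go to the possessed object while IsPossessing is set, otherwise to the character.
; Possess, unpossess and interact call the character, with the latter two only while possessing, so the controller itself never switches pawns.
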(event EventBeginPlay
  (CallFunction|SetReftoCharacter)
  (CallFunction|SetInputMappingContext "/Game/Inputs/IMC_Default.IMC_Default"))

(event Input|EnhancedActionEvents|EnhancedInputActionIA_Move
  (params (ActionValue :type Vector%202D%20Structure) (ElapsedSeconds :type Float%20%28double-precision%29) (TriggeredSeconds :type Float%20%28double-precision%29) (InputAction :type Input%20Action%20Object%20Reference :default "/Game/Inputs/Actions/IA_Move.IA_Move"))
  (bind _reftocharacter (Variables|Default|GetRefToCharacter))
  ;[0.15 0.15 0.15 0.5] Handle character movement inputs
  (if (Variables|/Game/Blueprints/Gamemode/Core/BP_Core_Character.BP_Core_Character_C|GetIsPossessing? _reftocharacter)
    (Default|Move (Variables|/Game/Blueprints/Gamemode/Core/BP_Core_Character.BP_Core_Character_C|GetRefToPossessedObject _reftocharacter) (.x ActionValue) (.y ActionValue))
    (else
      (Default|Move _reftocharacter (.x ActionValue) (.y ActionValue)))))

(event Input|EnhancedActionEvents|EnhancedInputActionIA_Look
  (params (ActionValue :type Vector%202D%20Structure) (ElapsedSeconds :type Float%20%28double-precision%29) (TriggeredSeconds :type Float%20%28double-precision%29) (InputAction :type Input%20Action%20Object%20Reference :default "/Game/Inputs/Actions/IA_Look.IA_Look"))
  (bind _reftocharacter (Variables|Default|GetRefToCharacter))
  ;[0.15 0.15 0.15 0.5] Handle character camera movement inputs
  (if (Variables|/Game/Blueprints/Gamemode/Core/BP_Core_Character.BP_Core_Character_C|GetIsPossessing? _reftocharacter)
    (Default|Look (Variables|/Game/Blueprints/Gamemode/Core/BP_Core_Character.BP_Core_Character_C|GetRefToPossessedObject _reftocharacter) (.x ActionValue) (.y ActionValue))
    (else
      (Default|Look _reftocharacter (.x ActionValue) (.y ActionValue)))))

(event Input|EnhancedActionEvents|EnhancedInputActionIA_Jump
  (params (ActionValue :type Boolean) (ElapsedSeconds :type Float%20%28double-precision%29) (TriggeredSeconds :type Float%20%28double-precision%29) (InputAction :type Input%20Action%20Object%20Reference :default "/Game/Inputs/Actions/IA_Jump.IA_Jump"))
  (bind _reftocharacter (Variables|Default|GetRefToCharacter))
  (bind _ispossessing_ (Variables|/Game/Blueprints/Gamemode/Core/BP_Core_Character.BP_Core_Character_C|GetIsPossessing? _reftocharacter))
  ;[0.15 0.15 0.15 0.5] Handle jump input
  (:Started
    (if _ispossessing_
      (Default|Jump (Variables|/Game/Blueprints/Gamemode/Core/BP_Core_Character.BP_Core_Character_C|GetRefToPossessedObject _reftocharacter))
      (else
        (Character|Jump _reftocharacter))))
  (:Completed
    (if (not _ispossessing_)
      (Character|StopJumping _reftocharacter))))

(event Input|EnhancedActionEvents|EnhancedInputActionIA_Possess
  (params (ActionValue :type Boolean) (ElapsedSeconds :type Float%20%28double-precision%29) (TriggeredSeconds :type Float%20%28double-precision%29) (InputAction :type Input%20Action%20Object%20Reference :default "/Game/Inputs/Actions/IA_Possess.IA_Possess"))
  ;[0.15 0.15 0.15 0.5] Handle the inputs to possess objects
  (:Started
    (Default|PossessObject (Variables|Default|GetRefToCharacter))))

(event Input|EnhancedActionEvents|EnhancedInputActionIA_Unpossess
  (params (ActionValue :type Boolean) (ElapsedSeconds :type Float%20%28double-precision%29) (TriggeredSeconds :type Float%20%28double-precision%29) (InputAction :type Input%20Action%20Object%20Reference :default "/Game/Inputs/Actions/IA_Unpossess.IA_Unpossess"))
  (bind _reftocharacter (Variables|Default|GetRefToCharacter))
  ;[0.15 0.15 0.15 0.5] Handle the inputs to unpossess objects
  (:Started
    (if (Variables|/Game/Blueprints/Gamemode/Core/BP_Core_Character.BP_Core_Character_C|GetIsPossessing? _reftocharacter)
      (Default|UnpossessObject _reftocharacter))))

(event Input|EnhancedActionEvents|EnhancedInputActionIA_Interact
  (params (ActionValue :type Boolean) (ElapsedSeconds :type Float%20%28double-precision%29) (TriggeredSeconds :type Float%20%28double-precision%29) (InputAction :type Input%20Action%20Object%20Reference :default "/Game/Inputs/Actions/IA_Interact.IA_Interact"))
  (bind _reftocharacter (Variables|Default|GetRefToCharacter))
  ;[0.15 0.15 0.15 0.5] Handle the inputs to interact with objects
  (:Started
    (if (Variables|/Game/Blueprints/Gamemode/Core/BP_Core_Character.BP_Core_Character_C|GetIsPossessing? _reftocharacter)
      (Default|Interact _reftocharacter))))

(fn ConstructionScript)

(fn SetReftoCharacter
  (bind _asbp_core_character (Utilities|Casting|CastToBP_Core_Character (Game|GetPlayerCharacter 0)))
  (Variables|Default|SetRefToCharacter _asbp_core_character))

(fn SetInputMappingContext
  (params (InputMappingContext :type Input%20Mapping%20Context%20Object%20Reference))
  (Input|AddMappingContext (PlayerController|LocalPlayerSubsystems|GetEnhancedInputLocalPlayerSubsystem self) InputMappingContext 0 "(bIgnoreAllPressedKeysUntilRelease=True,bForceImmediately=False,bNotifyUserSettings=False)"))