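; Player status component that tracks HP, applying damage and restoring health after a delay.
; TakeDamage subtracts damage, blocks healing and sets a timer intended to start Heal a few seconds later.
; Heal re-enables healing and adds HealStep in a while loop with no delay until HP reaches the hard-coded cap, then clears the timer handle.
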(event EventHeal
  ;[0.15 0.15 0.15 0.5] Until the player can heal, HP is increased by a heal step
  (Variables|Default|SetCanHeal? true)
  (while (and (Variables|Default|GetCanHeal?) (< (Variables|Default|GetHP) 1e+02))
    (Variables|Default|SetHP (+ (Variables|Default|GetHP) (Variables|Default|GetHealStep))))
  (Utilities|Time|ClearandInvalidateTimerbyHandle (Variables|Default|GetTimerHandle)))

(event EventTakeDamage
  (params (Damage :type Float%20%28double-precision%29))
  ;[0.15 0.15 0.15 0.5] Apply damage to HP and start a timer for starting Heal event
  (Variables|Default|SetCanHeal? false)
  (Variables|Default|SetHP (- (Variables|Default|GetHP) Damage))
  (bind _returnvalue (Utilities|Time|SetTimerbyEvent (EventDispatchers|CreateEvent :!event Heal) 5.0))
  (Variables|Default|SetTimerHandle _returnvalue))