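; Player status component that tracks HP and stamina and broadcasts changes, death and out-of-stamina through dispatchers.
; Taking damage or consuming stamina lowers the value, clamped at zero, and sets a delayed looping timer for regeneration, except on death.
; Healing adds a fixed step per tick, while stamina recovery speeds up the emptier it is.
; Both regenerate up to a hardcoded 100 rather than their max variables, then clear their timers.
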(event EventBeginPlay
  (Variables|Default|SetHP (Variables|Default|GetHPMax))
  (Variables|Default|SetStamina (Variables|Default|GetStaminaMax)))

(event EventHeal
  ;[0.15 0.15 0.15 0.5] Until the player can heal, HP is increased by a heal step
  (Variables|Default|SetCanHeal? true)
  (if (and (Variables|Default|GetCanHeal?) (< (Variables|Default|GetHP) 1e+02))
    (Variables|Default|SetHP (Math|Float|SelectFloat (+ (Variables|Default|GetHP) (Variables|Default|GetHealStep)) 1e+02 (< (+ (Variables|Default|GetHP) (Variables|Default|GetHealStep)) 1e+02)))
    (Default|CallOnHPChange)
    (else
      (Utilities|Time|ClearandInvalidateTimerbyHandle (Variables|Default|GetHealTimerHandle)))))

(event EventTakeDamage
  (params (Damage :type Float%20%28double-precision%29))
  ;[0.15 0.15 0.15 0.5] Apply damage to HP and start a timer for starting Heal event
  (Variables|Default|SetCanHeal? false)
  (bind _output_get (Variables|Default|SetHP (Math|Float|SelectFloat (- (Variables|Default|GetHP) Damage) 0.0 (> (- (Variables|Default|GetHP) Damage) 0.0))))
  (Default|CallOnHPChange)
  (if (> _output_get 0.0)
    (bind _returnvalue (Utilities|Time|SetTimerbyEvent (EventDispatchers|CreateEvent :!event Heal) 0.2 true false (Variables|Default|GetHealDelay)))
    (Variables|Default|SetHealTimerHandle _returnvalue)
    (else
      (Default|CallOnDeath))))

(event EventRecoverStamina
  ;[0.15 0.15 0.15 0.5] As long as the player isn’t consuming stamina, RecoverStamina is called by the timer, restoring a small amount of stamina each tick
  (Variables|Default|SetCanRecoverStamina? true)
  (if (and (Variables|Default|GetCanRecoverStamina?) (< (Variables|Default|GetStamina) 1e+02))
    (Variables|Default|SetStamina (Math|Float|SelectFloat (+ (Variables|Default|GetStamina) (+ (Variables|Default|GetStaminaRecoverStep) (* (- 1e+02 (Variables|Default|GetStamina)) 0.01))) 1e+02 (< (+ (Variables|Default|GetStamina) (+ (Variables|Default|GetStaminaRecoverStep) (* (- 1e+02 (Variables|Default|GetStamina)) 0.01))) 1e+02)))
    (Default|CallOnStaminaChange)
    (else
      (Utilities|Time|ClearandInvalidateTimerbyHandle (Variables|Default|GetStaminaTimerHandle)))))

(event EventConsumeStamina
  (params (StaminaModifier :type Float%20%28double-precision%29) (StaminaStep :type Float%20%28double-precision%29))
  ;[0.15 0.15 0.15 0.5] When the player is sprinting, or when a possessed object is walking or sprinting, stamina is consumed. If stamina hasn't been consumed for a certain amount of time, RecoverStamina is called
  (Variables|Default|SetCanRecoverStamina? false)
  (bind _output_get (Variables|Default|SetStamina (Math|Float|SelectFloat (- (Variables|Default|GetStamina) (* StaminaModifier StaminaStep)) 0.0 (> (- (Variables|Default|GetStamina) (* StaminaModifier StaminaStep)) 0.0))))
  (Default|CallOnStaminaChange)
  (if (== _output_get 0.0)
    (Default|CallOutOfStamina))
  (bind _returnvalue (Utilities|Time|SetTimerbyEvent (EventDispatchers|CreateEvent :!event RecoverStamina) 0.2 true false (Variables|Default|GetStaminaRecoveryDelay)))
  (Variables|Default|SetStaminaTimerHandle _returnvalue))