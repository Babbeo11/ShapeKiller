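; BPC_PlayerUI is a player UI component that shows health and stamina bars on screen.
; On BeginPlay it creates a WBP_StatusBars widget, fills both bars and adds it to the viewport.
; UpdateHealth and UpdateStamina events take a percent and set it directly on the matching progress bar.
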(event Custom|UpdateStamina
  (params (StaminaPercent :type Float%20%28double-precision%29))
  (Progress|SetPercent (Variables|/Game/Blueprints/UI/WBP_StatusBars.WBP_StatusBars_C|GetStaminaBar (Variables|Default|GetStatusWidget)) StaminaPercent))

(event Custom|UpdateHealth
  (params (HealthPercent :type Float%20%28double-precision%29))
  (Progress|SetPercent (Variables|/Game/Blueprints/UI/WBP_StatusBars.WBP_StatusBars_C|GetHealthBar (Variables|Default|GetStatusWidget)) HealthPercent))

(event EventBeginPlay
  (bind _returnvalue (UserInterface|CreateWidget "/Game/Blueprints/UI/WBP_StatusBars.WBP_StatusBars_C"))
  (bind _output_get (Variables|Default|SetStatusWidget _returnvalue))
  (CallFunction|UpdateHealth 1.0)
  (CallFunction|UpdateStamina 1.0)
  (UserInterface|Viewport|AddtoViewport _output_get 0))